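; Player controller that routes jump, movement and look input to the BP_Player pawn, which it casts and caches on BeginPlay.
; Movement input follows the player camera's forward and right vectors, with axis values scaled up before being applied.
; Turn feeds yaw directly, while LookUp adds pitch only if the predicted control rotation stays within an allowed window, handling the 360-degree wrap to limit vertical look.
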(event `self.ReceiveBeginPlay`
  (bind _asbp_player (cast `/Game/Blueprint/Characters/Player/BP_Player` (`self.K2_GetPawn`)))
  (set `self.PlayerRef` _asbp_player))

(event `InputAction|Jump`
  (params (Key :type "Key Structure"))
  (:`Pressed`
    (`Character.Jump` (`self.PlayerRef`))))

(event `InputAxis|MoveForward`
  (params (AxisValue :type "Float (single-precision)"))
  (bind _playerref (`self.PlayerRef`))
  (`Pawn.AddMovementInput` _playerref (`SceneComponent.GetForwardVector` (`/Game/Blueprint/Characters/Player/BP_Player.Camera` _playerref)) (* AxisValue 100.0) false))

(event `InputAxis|MoveRight`
  (params (AxisValue :type "Float (single-precision)"))
  (bind _playerref (`self.PlayerRef`))
  (`Pawn.AddMovementInput` _playerref (`SceneComponent.GetRightVector` (`/Game/Blueprint/Characters/Player/BP_Player.Camera` _playerref)) (* AxisValue 100.0) false))

(event `InputAxis|Turn`
  (params (AxisValue :type "Float (single-precision)"))
  (`self.AddYawInput` AxisValue))

(event `InputAxis|LookUp`
  (params (AxisValue :type "Float (single-precision)"))
  (bind (_returnvalue_roll _returnvalue_pitch) (`KismetMathLibrary.BreakRotator` (`self.GetControlRotation`)))
  (bind _returnvalue (+ _returnvalue_pitch (* AxisValue (`self.InputPitchScale`))))
  (if (or (and (> _returnvalue 300.0) (< _returnvalue 999.0)) (and (< _returnvalue 45.0) (> _returnvalue -999.0)))
    (`self.AddPitchInput` AxisValue)))

(fn `UserConstructionScript`)